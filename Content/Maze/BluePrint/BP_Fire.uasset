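; BP_Fire is a fire hazard actor in the Maze game that damages the player character while it stands inside the fire's box.
; Box begin overlap casts to BP_ThirdPerson, stores the reference, sets OnFire and calls the Burn event.
; Burn applies damage at once, then repeats every half second through a looped Delay until end overlap clears OnFire.
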(event `self.ReceiveBeginPlay`)

(event `self.ReceiveTick`
  (params (DeltaSeconds :type "Float (single-precision)")))

(event `self.Box.OnComponentBeginOverlap`
  (params (OverlappedComponent :type "PrimitiveComponent Object Reference") (OtherActor :type "Actor Object Reference") (OtherComp :type "PrimitiveComponent Object Reference") (OtherBodyIndex :type Integer) (bFromSweep :type Boolean) (SweepResult :type "HitResult Structure (by ref)"))
  (bind _asbp_third_person (cast `/Game/ThirdPerson/Blueprints/BP_ThirdPerson` OtherActor))
  (set `self.As BP Third Person Character` _asbp_third_person)
  (set `self.OnFire` true)
  (`self.Burn`))

(event `self.Box.OnComponentEndOverlap`
  (params (OverlappedComponent :type "PrimitiveComponent Object Reference") (OtherActor :type "Actor Object Reference") (OtherComp :type "PrimitiveComponent Object Reference") (OtherBodyIndex :type Integer))
  (cast `/Game/ThirdPerson/Blueprints/BP_ThirdPerson` OtherActor)
  (set `self.OnFire` false))

(event `Burn`
  (if (`self.OnFire`) :!label _label
    (`/Game/ThirdPerson/Blueprints/BP_ThirdPerson.TakeDamage` (`self.As BP Third Person Character`) 5.0)
    (`KismetSystemLibrary.Delay` 0.5)
    (goto _label)))

(fn `UserConstructionScript`)