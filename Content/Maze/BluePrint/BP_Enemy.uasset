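; BP_Enemy is a stationary maze turret that tracks and shoots the player inside its detection sphere.
; Sphere overlaps with BP_ThirdPerson toggle InRange and start the loop on entry.
; A zero-delay loop replaces Tick, rotating the Arrow toward player zero at constant speed.
; Each pass also hits a short Delay, which ignores retriggers while pending, throttling BP_Bullet spawns at PSpawnLocation into steady fire.
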(event `self.ReceiveTick`
  (params (DeltaSeconds :type "Float (single-precision)")))

(event `StartLoop`
  (bind _arrow (`self.Arrow`))
  (bind _pspawnlocation (`self.PSpawnLocation`))
  (if (`self.InRange`) :!label _label
    (`SceneComponent.K2_SetWorldRotation` (`self.Arrow`) (`KismetMathLibrary.RInterpTo_Constant` (`SceneComponent.K2_GetComponentRotation` _arrow) (`KismetMathLibrary.FindLookAtRotation` (`SceneComponent.K2_GetComponentLocation` _arrow) (`SceneComponent.K2_GetComponentLocation` (`Character.CapsuleComponent` (`GameplayStatics.GetPlayerCharacter` 0)))) (`GameplayStatics.GetWorldDeltaSeconds`) 100.0) false false)
    (`KismetSystemLibrary.Delay` 0.0)
    (`|ExecutionSequence`
      (:`then_0`
        (goto _label))
      (:`then_1`
        (`KismetSystemLibrary.Delay` 0.3)
        (`|SpawnActorFromClass` "/Game/Maze/BluePrint/BP_Bullet.BP_Bullet_C" (`KismetMathLibrary.MakeTransform` (`SceneComponent.K2_GetComponentLocation` _pspawnlocation) (`SceneComponent.K2_GetComponentRotation` _pspawnlocation)) "AdjustIfPossibleButAlwaysSpawn" "MultiplyWithRoot" null null)))))

(event `self.Sphere.OnComponentBeginOverlap`
  (params (OverlappedComponent :type "PrimitiveComponent Object Reference") (OtherActor :type "Actor Object Reference") (OtherComp :type "PrimitiveComponent Object Reference") (OtherBodyIndex :type Integer) (bFromSweep :type Boolean) (SweepResult :type "HitResult Structure (by ref)"))
  (cast `/Game/ThirdPerson/Blueprints/BP_ThirdPerson` OtherActor)
  (set `self.InRange` true)
  (`self.StartLoop`))

(event `self.Sphere.OnComponentEndOverlap`
  (params (OverlappedComponent :type "PrimitiveComponent Object Reference") (OtherActor :type "Actor Object Reference") (OtherComp :type "PrimitiveComponent Object Reference") (OtherBodyIndex :type Integer))
  (cast `/Game/ThirdPerson/Blueprints/BP_ThirdPerson` OtherActor)
  (set `self.InRange` false))

(fn `UserConstructionScript`)