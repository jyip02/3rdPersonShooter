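; Actor component for a pawn, an unfinished box-placement check for the Maze game that only performs a debug-drawn trace.
; TryPutBox line-traces on Visibility from the owning pawn's location over TraceDistance, discarding the result.
; The direction takes only control-rotation roll, with pitch and yaw zeroed, so it always points along world +X.
; BeginPlay and Tick do nothing; a duplicate trace in the event graph is unconnected.
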(event `self.ReceiveTick`
  (params (DeltaSeconds :type "Float (single-precision)")))

(fn `_GetPawnOwner`
  (returns (PawnOwner :type "Pawn Object Reference"))
  (bind _aspawn (cast `Pawn` (`self.GetOwner`)))
  (return _aspawn))

(fn `TryPutBox`
  (bind _pawnowner (`self._GetPawnOwner`))
  (bind _returnvalue (`Actor.K2_GetActorLocation` _pawnowner))
  (bind _returnvalue_roll (`KismetMathLibrary.BreakRotator` (`Pawn.GetControlRotation` _pawnowner)))
  (`KismetSystemLibrary.LineTraceSingle` :`Start` (+ _returnvalue (0.0 0.0 0.0)) :`End` (+ _returnvalue (* (`KismetMathLibrary.GetForwardVector` (`KismetMathLibrary.MakeRotator` _returnvalue_roll)) (`self.TraceDistance`))) :`TraceChannel` "TraceTypeQuery1" :`DrawDebugType` "ForOneFrame" :`TraceColor` (struct :`G` 0.537807 :`B` 1.0 :`A` 1.0) :`TraceHitColor` (struct :`R` 0.152777 :`B` 1.0 :`A` 1.0)))