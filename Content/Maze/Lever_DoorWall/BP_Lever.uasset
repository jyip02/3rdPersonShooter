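; BP_Lever is a maze lever that toggles between down and up states and opens a linked door wall.
; Each ActivateLever call alternates through a FlipFlop, swapping the lever's static mesh, setting LeverActivated and printing ON or OFF.
; Switching on casts the Door reference to BP_DoorWall and calls OpenDoor; switching off leaves the door untouched.
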(event `ActivateLever`
  (bind _door (`self.Door`))
  (`/Engine/EditorBlueprintResources/StandardMacros.FlipFlop`
    (:`A`
      (`StaticMeshComponent.SetStaticMesh` (`self.StaticMesh`) "/Game/Maze/Lever_DoorWall/SM_Level_DOWN.SM_Level_DOWN")
      (set `self.bLeverActivated` true)
      (`KismetSystemLibrary.PrintString` "ON")
      (if (`self.bLeverActivated`)
        (cast `/Game/Maze/Lever_DoorWall/BP_DoorWall` _door)
        (`/Game/Maze/Lever_DoorWall/BP_DoorWall.OpenDoor` _door)))
    (:`B`
      (`StaticMeshComponent.SetStaticMesh` (`self.StaticMesh`) "/Game/Maze/Lever_DoorWall/SM_Lever_UP.SM_Lever_UP")
      (set `self.bLeverActivated` false)
      (`KismetSystemLibrary.PrintString` "OFF"))))

(fn `UserConstructionScript`)