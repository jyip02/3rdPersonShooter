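; BP_HealingBall is a health pickup that restores HP to the BP_ThirdPerson character on touch.
; A Sphere overlap event casts the overlapping actor and ignores anything that is not that character.
; It calls Heal with AmountOfHealing, or sets CurrentHP directly to a hardcoded cap of 100 when the heal would reach or exceed it.
; The ball destroys itself after either outcome, even if the character is already at full health.
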(event `self.Sphere.OnComponentBeginOverlap`
  (params (OverlappedComponent :type "PrimitiveComponent Object Reference") (OtherActor :type "Actor Object Reference") (OtherComp :type "PrimitiveComponent Object Reference") (OtherBodyIndex :type Integer) (bFromSweep :type Boolean) (SweepResult :type "HitResult Structure (by ref)"))
  (bind _asbp_third_person (cast `/Game/ThirdPerson/Blueprints/BP_ThirdPerson` OtherActor))
  (if (>= (+ (`/Game/ThirdPerson/Blueprints/BP_ThirdPerson.CurrentHP` _asbp_third_person) (`self.Amount Of Healing`)) 100.0)
    (set `/Game/ThirdPerson/Blueprints/BP_ThirdPerson.CurrentHP` 100.0 _asbp_third_person)
    (`self.K2_DestroyActor`)
    (else
      (`/Game/ThirdPerson/Blueprints/BP_ThirdPerson.heal` _asbp_third_person (`self.Amount Of Healing`))
      (`self.K2_DestroyActor`))))

(fn `UserConstructionScript`)